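; BP_Footballer is a footballer that picks up a BP_Ball on contact, dribbles it and passes it with the X key.
; Overlapping BallAlert starts dribbling by hiding the ball, disabling its physics and showing the footballer's own Sphere as a stand-in.
; Passing hides that Sphere, spawns a new ball there with a forward PassPower impulse, and briefly blocks recapture through Shot.
; The original ball is stored in TempBall, not destroyed.
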(event `self.ReceiveTick`
  (params (DeltaSeconds :type "Float (single-precision)")))

(event `self.BallAlert.OnComponentBeginOverlap`
  (params (OverlappedComponent :type "PrimitiveComponent Object Reference") (OtherActor :type "Actor Object Reference") (OtherComp :type "PrimitiveComponent Object Reference") (OtherBodyIndex :type Integer) (bFromSweep :type Boolean) (SweepResult :type "HitResult Structure (by ref)"))
  (if (not (`self.shot?`))
    (bind _asbp_ball (cast `/Game/Footballer/BP_Ball` OtherActor))
    (bind _output_get (set `self.Ball` _asbp_ball))
    (set `self.IsDribbling?` true)
    (`SceneComponent.SetHiddenInGame` (`self.Sphere`) false false)
    (bind _sphere (`/Game/Footballer/BP_Ball.Sphere` _output_get))
    (`SceneComponent.SetHiddenInGame` _sphere true false)
    (`PrimitiveComponent.SetSimulatePhysics` _sphere false)))

(event `Key|X`
  (params (Key :type "Key Structure"))
  (bind _sphere (`self.Sphere`))
  (:`Pressed`
    (if (`self.IsDribbling?`)
      (set `self.IsDribbling?` false)
      (`SceneComponent.SetHiddenInGame` _sphere true false)
      (bind _returnvalue (`|SpawnActorFromClass` (`GameplayStatics.GetObjectClass` (`self.Ball`)) (`KismetMathLibrary.MakeTransform` (`SceneComponent.K2_GetComponentLocation` _sphere) (`SceneComponent.K2_GetComponentRotation` _sphere)) "Undefined" "MultiplyWithRoot" null null))
      (set `self.tempBall` (`self.Ball`))
      (set `self.Ball` _returnvalue)
      (bind _sphere_2 (`/Game/Footballer/BP_Ball.Sphere` _returnvalue))
      (`PrimitiveComponent.SetSimulatePhysics` _sphere_2 true)
      (`PrimitiveComponent.AddImpulse` _sphere_2 (* (`SceneComponent.GetForwardVector` (`self.CapsuleComponent`)) (`self.PassPower`)) "None" false)
      (set `self.shot?` true)
      (`KismetSystemLibrary.Delay` 0.2)
      (set `self.shot?` false))))

(fn `UserConstructionScript`
  (`parent.UserConstructionScript`))